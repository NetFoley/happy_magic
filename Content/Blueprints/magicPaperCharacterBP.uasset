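; Paper2D side-view character Blueprint for a wizard moved by player axis input.
; Up/Down input moves it along world Z and Right/left along world X.
; Each tick it stores the last horizontal input direction and swaps the sprite's flipbook between run and idle, based on whether velocity is non-zero.
; Left and right facings use separate flipbooks rather than a flipped sprite.
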(event `InputAxis|Up/Down`
  (params (AxisValue :type "Float (single-precision)"))
  (`self.AddMovementInput` (0.0 0.0 1.0) AxisValue))

(event `InputAxis|Right/left`
  (params (AxisValue :type "Float (single-precision)"))
  (`self.AddMovementInput` (1.0 0.0 0.0) AxisValue))

(event `self.ReceiveTick`
  (params (DeltaSeconds :type "Float (single-precision)"))
  (`self.updateFlipbook`))

(fn `updateFlipbook`
  (bind _lastmovedirection (`self.lastMoveDirection`))
  (if (!= (`self.GetInputAxisValue`) 0.0)
    (set `self.lastMoveDirection` (select `bool` (> (`self.GetInputAxisValue`) 0.0) :`false` "NewEnumerator0" :`true` "NewEnumerator1" :!type "/Game/assets/characters/moveDirection Enum")))
  (`PaperFlipbookComponent.SetFlipbook` (`self.Sprite`) (select `bool` (> (`KismetMathLibrary.VSize` (`self.GetVelocity`)) 0.0) :`false` (select `/Game/assets/characters/moveDirection` _lastmovedirection :`NewEnumerator0` "/Game/assets/characters/wizardIdleL.wizardIdleL" :`NewEnumerator1` "/Game/assets/characters/wizzardIdle.wizzardIdle" :!type "PaperFlipbook Object Reference") :`true` (select `/Game/assets/characters/moveDirection` _lastmovedirection :`NewEnumerator0` "/Game/assets/characters/wizardRunL.wizardRunL" :`NewEnumerator1` "/Game/assets/characters/wizardRun.wizardRun" :!type "PaperFlipbook Object Reference"))))

(fn `UserConstructionScript`)